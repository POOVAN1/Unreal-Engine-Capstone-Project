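; BP_InvisibleWall is a wall actor that reveals part of itself when the player comes near.
; Player overlap with DetectionSphere, checked through INT_Player, plays a timeline that fades the dynamic material's Opacity up to a partial value, and reverses it on exit.
; Tick feeds the player's location to the material's PlayerPosition parameter every frame, regardless of proximity.
; PlayerNearby is set on overlap changes but not read here.
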(event `self.ReceiveBeginPlay`
  ;[0 0 0 0.5] Set Wall Material
  (set `self.PlayerREF` (`GameplayStatics.GetPlayerCharacter` 0))
  (bind _returnvalue (`PrimitiveComponent.CreateDynamicMaterialInstance` (`self.WallMesh`) 0 "/Game/Main/InvisibleWall/M_InvisibleWall.M_InvisibleWall" "None"))
  (set `self.WallMaterial` _returnvalue))

(event `self.DetectionSphere.OnComponentBeginOverlap`
  (params (OverlappedComponent :type "PrimitiveComponent Object Reference") (OtherActor :type "Actor Object Reference") (OtherComp :type "PrimitiveComponent Object Reference") (OtherBodyIndex :type Integer) (bFromSweep :type Boolean) (SweepResult :type "HitResult Structure (by ref)"))
  ;[0 0 0 0.5] Show part of the wall to player on overlap.
  (if (`KismetSystemLibrary.DoesImplementInterface` OtherActor "/Game/Main/Interfaces/INT_Player.INT_Player_C")
    (set `self.PlayerNearby` true)
    (bind (_direction _fade) (`Timeline|TL_WallFade` :!label _label)
      (:`Update`
        (`MaterialInstanceDynamic.SetScalarParameterValue` (`self.WallMaterial`) "Opacity" (`KismetMathLibrary.Lerp` 0.0 0.35 _fade))))))

(event `self.DetectionSphere.OnComponentEndOverlap`
  (params (OverlappedComponent :type "PrimitiveComponent Object Reference") (OtherActor :type "Actor Object Reference") (OtherComp :type "PrimitiveComponent Object Reference") (OtherBodyIndex :type Integer))
  ;[0 0 0 0.5] Don't show wall if player loses contact with detection sphere
  (if (`KismetSystemLibrary.DoesImplementInterface` OtherActor "/Game/Main/Interfaces/INT_Player.INT_Player_C")
    (set `self.PlayerNearby` false)
    (goto _label :!via `Reverse`)))

(event `self.ReceiveTick`
  (params (DeltaSeconds :type "Float (single-precision)"))
  ;[0 0 0 0.5] Update wall visibility based on player distance to wall
  (`MeshComponent.SetVectorParameterValueOnMaterials` (`self.WallMesh`) "PlayerPosition" (`self.K2_GetActorLocation` (`self.PlayerREF`))))

(fn `UserConstructionScript`)