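; Player controller for the spaceship game that sets up Enhanced Input and owns the HUD.
; On BeginPlay it adds the spaceship mapping context, shows the mouse cursor and creates the WB_HUD widget.
; Custom events forward lives, score and wave-end screen open and close updates to the HUD.
; Each retries on the next frame until the HUD is valid, covering calls that arrive before it exists.
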(event `self.ReceiveBeginPlay`
  (bind _returnvalue (subsystem `EnhancedInputLocalPlayerSubsystem`))
  (`/Engine/EditorBlueprintResources/StandardMacros.IsValid` _returnvalue
    (:`Is Valid`
      (`EnhancedInputSubsystemInterface.AddMappingContext` _returnvalue "/Game/Main/Player/Input/IMC_SpaceShip.IMC_SpaceShip" 0 (struct))
      (set `PlayerController.bShowMouseCursor` true (`GameplayStatics.GetPlayerController` 0))
      (bind _returnvalue_2 (`|CreateWidget` "/Game/Main/HUD/WB_HUD.WB_HUD_C" self))
      (bind _output_get (set `self.HUD` _returnvalue_2))
      (`UserWidget.AddToViewport` _output_get 0))))

(event `/Game/Main/Interfaces/INT_PlayerController.UpdateLives`
  (params (Lives :type Integer))
  (bind _hud (`self.HUD` :!label _label)
    (:`then`
      (`/Game/Main/HUD/WB_HUD.LoseLife` _hud Lives))
    (:`else`
      (`KismetSystemLibrary.DelayUntilNextFrame`)
      (goto _label))))

(event `/Game/Main/Interfaces/INT_PlayerController.UpdateScore`
  (params (CurrentScore :type Integer) (TotalScore :type Integer))
  (bind _hud (`self.HUD` :!label _label_2)
    (:`then`
      (`/Game/Main/HUD/WB_HUD.UpdateScore` _hud CurrentScore TotalScore))
    (:`else`
      (`KismetSystemLibrary.DelayUntilNextFrame`)
      (goto _label_2))))

(event `/Game/Main/Interfaces/INT_PlayerController.UpdateShowWaveEndScreen`
  (params (TotalScore :type Integer) (GoalTime :type Integer) (PlayerTime :type Integer) (TimeBonus :type Integer) (CurrentWave :type Integer))
  (bind _hud (`self.HUD` :!label _label_3)
    (:`then`
      (`/Game/Main/HUD/WB_HUD.ShowWaveCompletedScreen` _hud 0 TotalScore GoalTime PlayerTime TimeBonus CurrentWave))
    (:`else`
      (`KismetSystemLibrary.DelayUntilNextFrame`)
      (goto _label_3))))

(event `/Game/Main/Interfaces/INT_PlayerController.UpdateCloseWaveEndScreen`
  (params (CloseScreen :type Boolean))
  (bind _hud (`self.HUD` :!label _label_4)
    (:`then`
      (`/Game/Main/HUD/WB_HUD.CloseWaveEndScreen` _hud CloseScreen))
    (:`else`
      (`KismetSystemLibrary.DelayUntilNextFrame`)
      (goto _label_4))))

(fn `UserConstructionScript`)