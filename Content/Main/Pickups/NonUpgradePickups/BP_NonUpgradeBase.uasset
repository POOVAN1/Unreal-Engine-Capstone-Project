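; Base Blueprint for non-upgrade pickups that drift horizontally while their mesh spins.
; BeginPlay randomizes spin speed; only on a coin-flip success does it reverse spin, pick a random drift speed and direction, and start the PulseScale timeline that drives mesh scale.
; Tick applies drift as an unswept world offset and rolls UpgradeMesh, both scaled by delta time.
; No overlap or collection logic is implemented here.
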(event `self.ReceiveBeginPlay`
  (set `self.RotationSpeed` (`KismetMathLibrary.RandomFloatInRange` 20.0 80.0))
  (if (`KismetMathLibrary.RandomBool`)
    (set `self.RotationSpeed` (* (`self.RotationSpeed`) -1.0))
    (set `self.MovementSpeed` (`KismetMathLibrary.RandomFloatInRange` 400.0 600.0))
    (set `self.MovementDirection` (`KismetMathLibrary.Normal` (`KismetMathLibrary.MakeVector` (`KismetMathLibrary.RandomFloatInRange` -1.0 1.0) (`KismetMathLibrary.RandomFloatInRange` -1.0 1.0))))
    (bind (_direction _scale) (`Timeline|PulseScale` :!via `PlayFromStart`)
      (:`Update`
        (bind _output_get (set `self.Scale` _scale))
        (`SceneComponent.SetRelativeScale3D` (`self.UpgradeMesh`) (`KismetMathLibrary.MakeVector` _output_get _output_get _output_get))))))

(event `self.ReceiveTick`
  (params (DeltaSeconds :type "Float (single-precision)"))
  (`self.K2_AddActorWorldOffset` (* (* (`self.MovementDirection`) (`self.MovementSpeed`)) (`GameplayStatics.GetWorldDeltaSeconds`)))
  (bind _upgrademesh (`self.UpgradeMesh`)
    (:`then`
      (`SceneComponent.K2_AddWorldRotation` _upgrademesh (`KismetMathLibrary.MakeRotator` (* (`self.RotationSpeed`) (`GameplayStatics.GetWorldDeltaSeconds`))) false false))
    (:`else`)))

(fn `UserConstructionScript`
  (`parent.UserConstructionScript`))