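; Base Blueprint for large asteroids, which break apart into smaller asteroids when destroyed.
; On death it spawns a random number of actors, each usually a small asteroid with a one-in-six chance of an upgrade asteroid.
; Each spawn is placed at a random offset along the asteroid's forward axis, then the parent's death handling runs.
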(event `self.HandleDeath`
  (bind _returnvalue (+ (`self.K2_GetActorLocation`) (* (`self.GetActorForwardVector`) (`KismetMathLibrary.RandomFloatInRange` -50.0 50.0))))
  (for _ (range (+ (`KismetMathLibrary.RandomIntegerInRange` 4 8) 1))
    (switch `int` (`KismetMathLibrary.RandomIntegerInRange` 0 5)
      (:`0`
        (`|SpawnActorFromClass` "/Game/Main/Asteroids/SmallAsteroids/BP_SmallAsteroidBase.BP_SmallAsteroidBase_C" (`KismetMathLibrary.MakeTransform` _returnvalue) "Undefined" "MultiplyWithRoot" null null :!label _label))
      (:`1`
        (goto _label))
      (:`2`
        (goto _label))
      (:`3`
        (goto _label))
      (:`4`
        (goto _label))
      (:`5`
        (`|SpawnActorFromClass` "/Game/Main/Asteroids/SmallAsteroids/BP_UpgradeAsteroid.BP_UpgradeAsteroid_C" (`KismetMathLibrary.MakeTransform` _returnvalue) "Undefined" "MultiplyWithRoot" null null))))
  (`parent.HandleDeath`))

(fn `UserConstructionScript`
  (`parent.UserConstructionScript`))