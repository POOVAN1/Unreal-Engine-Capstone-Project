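; BP_UpgradeAsteroid is a small asteroid that drops an upgrade when it dies.
; It overrides HandleDeath to spawn a BP_RockCrusherUpgrade at its location with a fixed rotation, then calls the parent death logic.
; A random three-way switch picks the drop, but every case leads to the same upgrade, so the result never varies.
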(event `/Game/Main/Asteroids/BP_AsteroidBase.HandleDeath`
  (switch `int` (`KismetMathLibrary.RandomIntegerInRange` 0 2)
    (:`0`
      _)
    (:`1`
      _)
    (:`2`
      _))
  (`|SpawnActorFromClass` "/Game/Main/Pickups/Upgrades/RockCrusherUpgrade/BP_RockCrusherUpgrade.BP_RockCrusherUpgrade_C" (`KismetMathLibrary.MakeTransform` (`self.K2_GetActorLocation`) (struct :`Yaw` -180.0)) "Undefined" "MultiplyWithRoot" null null)
  (`parent.HandleDeath`))

(fn `UserConstructionScript`
  (`parent.UserConstructionScript`))