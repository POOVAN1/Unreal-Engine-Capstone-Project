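; Asteroid spawner actor that periodically drops random asteroid pattern actors at random points inside its SpawnArea box.
; A looping timer started on BeginPlay randomly picks a small group, a large group or nothing.
; Small groups choose among three pattern Blueprints.
; Large groups have only pattern 01 wired, so their other two rolls spawn nothing.
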(event `self.ReceiveBeginPlay`
  (`KismetSystemLibrary.K2_SetTimerDelegate` (delegate `PickAsteroidPattern`) 3.0 true))

(event `PickAsteroidPattern`
  (bind _output_get (set `self.AsteroidPatternNumber` (`KismetMathLibrary.RandomIntegerInRange` 0 2)))
  (switch `int` _output_get
    (:`0`
      (`self.SpawnSmallAsteroidGroup`))
    (:`2`
      (`self.SpawnLargeAsteroidGroup`))))

(event `SpawnSmallAsteroidGroup`
  (bind _spawnarea (`self.SpawnArea`))
  (bind _spawnarea_2 (`self.SpawnArea`))
  (bind _spawnarea_3 (`self.SpawnArea`))
  (bind _output_get (set `self.AsteroidPatternNumber` (`KismetMathLibrary.RandomIntegerInRange` 0 2)))
  (switch `int` _output_get
    (:`0`
      (`|SpawnActorFromClass` "/Game/Main/Asteroids/SmallAsteroids/Patterns/BP_SmallAsteroidPattern01.BP_SmallAsteroidPattern01_C" (`KismetMathLibrary.MakeTransform` (`KismetMathLibrary.RandomPointInBoundingBox` (`SceneComponent.K2_GetComponentLocation` _spawnarea) (`BoxComponent.GetScaledBoxExtent` _spawnarea))) "Undefined" "MultiplyWithRoot" null null))
    (:`1`
      (`|SpawnActorFromClass` "/Game/Main/Asteroids/SmallAsteroids/Patterns/BP_SmallAsteroidPattern02.BP_SmallAsteroidPattern02_C" (`KismetMathLibrary.MakeTransform` (`KismetMathLibrary.RandomPointInBoundingBox` (`SceneComponent.K2_GetComponentLocation` _spawnarea_2) (`BoxComponent.GetScaledBoxExtent` _spawnarea_2))) "Undefined" "MultiplyWithRoot" null null))
    (:`2`
      (`|SpawnActorFromClass` "/Game/Main/Asteroids/SmallAsteroids/Patterns/BP_SmallAsteroidPattern03.BP_SmallAsteroidPattern03_C" (`KismetMathLibrary.MakeTransform` (`KismetMathLibrary.RandomPointInBoundingBox` (`SceneComponent.K2_GetComponentLocation` _spawnarea_3) (`BoxComponent.GetScaledBoxExtent` _spawnarea_3))) "Undefined" "MultiplyWithRoot" null null))))

(event `SpawnLargeAsteroidGroup`
  (bind _spawnarea (`self.SpawnArea`))
  (bind _output_get (set `self.AsteroidPatternNumber` (`KismetMathLibrary.RandomIntegerInRange` 0 2)))
  (switch `int` _output_get
    (:`0`
      (`|SpawnActorFromClass` "/Game/Main/Asteroids/LargeAsteroids/Patterns/BP_LargeAsteroidPattern01.BP_LargeAsteroidPattern01_C" (`KismetMathLibrary.MakeTransform` (`KismetMathLibrary.RandomPointInBoundingBox` (`SceneComponent.K2_GetComponentLocation` _spawnarea) (`BoxComponent.GetScaledBoxExtent` _spawnarea))) "Undefined" "MultiplyWithRoot" null null))))

(fn `UserConstructionScript`)