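; Base asteroid actor that descends, then drifts and spins once flagged as having reached the bottom.
; Tick moves it along the down direction until ChangeDirection sets that flag and picks a one-time random horizontal heading for swept movement.
; SpawnIndicator places a flashing landing indicator at a fixed height under a given location.
; Damage depletes health, triggering a small Niagara explosion and destroying the actor.
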(event `self.ReceiveBeginPlay`
  (set `self.RotationSpeed` (`KismetMathLibrary.RandomFloatInRange` 20.0 80.0))
  (if (`KismetMathLibrary.RandomBool`)
    (set `self.RotationSpeed` (* (`self.RotationSpeed`) -1.0))
    (set `self.MovementSpeed` (`KismetMathLibrary.RandomFloatInRange` 50.0 100.0))))

(event `self.ReceiveTick`
  (params (DeltaSeconds :type "Float (single-precision)"))
  (if (`self.HasReachedBottom`)
    (`self.K2_AddActorWorldOffset` (* (* (`self.MovementDirection`) (`self.MovementSpeed`)) (`GameplayStatics.GetWorldDeltaSeconds`)) true)
    (`self.K2_AddActorLocalRotation` (`KismetMathLibrary.MakeRotator` (* (`self.RotationSpeed`) (`GameplayStatics.GetWorldDeltaSeconds`))))
    (else
      (`self.K2_AddActorWorldOffset` (* (* (`self.MovementDownDirection`) (`self.MovementDownSpeed`)) (`GameplayStatics.GetWorldDeltaSeconds`))))))

(event `/Game/Main/Interfaces/INT_Asteroid.ChangeDirection`
  (params (ReachedBottom :type Boolean))
  (bind _output_get (set `self.HasReachedBottom` ReachedBottom))
  (if _output_get
    (`/Engine/EditorBlueprintResources/StandardMacros.DoOnce` false
      (:`Completed`
        (set `self.MovementDirection` (`KismetMathLibrary.Normal` (`KismetMathLibrary.MakeVector` (`KismetMathLibrary.RandomFloatInRange` -1.0 1.0) (`KismetMathLibrary.RandomFloatInRange` -1.0 1.0))))))))

(event `/Game/Main/Interfaces/INT_Asteroid.SpawnIndicator`
  (params (AsteroidLocation :type "Vector Structure"))
  (bind _returnvalue (`|SpawnActorFromClass` "/Game/Main/Enemies/EnemySpawnMarker/BP_LandingIndicator.BP_LandingIndicator_C" (`KismetMathLibrary.MakeTransform` (`KismetMathLibrary.MakeVector` (.x AsteroidLocation) (.y AsteroidLocation) 92.0)) "Undefined" "MultiplyWithRoot" null null))
  (`/Game/Main/Enemies/EnemySpawnMarker/BP_LandingIndicator.PlayFlash` _returnvalue))

(event `self.ReceiveAnyDamage`
  (params (Damage :type "Float (single-precision)") (DamageType :type "DamageType Object Reference") (InstigatedBy :type "Controller Object Reference") (DamageCauser :type "Actor Object Reference"))
  (if (not (`self.IsDead`))
    (set `self.Health` (- (`self.Health`) Damage))
    (if (<= (`self.Health`) 0.0)
      (set `self.IsDead` true)
      (`self.HandleDeath`))))

(event `HandleDeath`
  (`self.MultiPlayFX`)
  (`self.K2_DestroyActor`))

(event `MultiPlayFX`
  (`NiagaraFunctionLibrary.SpawnSystemAtLocation` "/Game/NiagaraExamples/FX_Explosions/NS_Explosion_Small.NS_Explosion_Small" (`self.K2_GetActorLocation`)))

(fn `UserConstructionScript`)