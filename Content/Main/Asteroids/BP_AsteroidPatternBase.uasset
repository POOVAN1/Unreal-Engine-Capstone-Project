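; Base actor for an asteroid pattern, grouping seven asteroid child actors.
; The construction script collects the child actor components into an array.
; On BeginPlay it caches the first BP_AsteroidBase found in the world, then calls SpawnIndicatorMessage on each child asteroid at its location.
; Tick is empty, and the speed-and-direction world offset logic for moving the pattern is disconnected.
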(event `self.ReceiveBeginPlay`
  (bind _returnvalue (`GameplayStatics.GetActorOfClass` "/Game/Main/Asteroids/BP_AsteroidBase.BP_AsteroidBase_C"))
  (bind _asbp_asteroid_base (cast `/Game/Main/Asteroids/BP_AsteroidBase` _returnvalue))
  (set `self.AsteroidBaseREF` _asbp_asteroid_base)
  (for _array_element (`self.Asteroids`)
    (bind _childactor (`ChildActorComponent.ChildActor` _array_element))
    (message `/Game/Main/Interfaces/INT_Asteroid.SpawnIndicator` _childactor (`self.K2_GetActorLocation` _childactor))))

(event `self.ReceiveTick`
  (params (DeltaSeconds :type "Float (single-precision)")))

(fn `UserConstructionScript`
  (set `self.Asteroids` (`|MakeArray` (`self.Asteroid01`) (`self.Asteroid02`) (`self.Asteroid03`) (`self.Asteroid04`) (`self.Asteroid05`) (`self.Asteroid06`) (`self.Asteroid07`))))