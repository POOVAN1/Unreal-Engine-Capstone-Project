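; Actor component that briefly flashes the owner's skeletal mesh when the owner takes damage.
; On BeginPlay it binds to OnTakeAnyDamage and creates dynamic material instances for every slot, saving one original emissive color and strength (last slot wins).
; DamageFlash sets EmissiveFactor and EmissiveStrength to the flash values, then after a Delay restores all materials to that saved pair.
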(event `self.ReceiveBeginPlay`
  (bind _returnvalue (`self.GetOwner`))
  (bind _returnvalue_2 (`Actor.GetComponentByClass` (`self.Owner`) "/Script/Engine.SkeletalMeshComponent"))
  (set `self.Owner` _returnvalue)
  (add `Actor.OnTakeAnyDamage` _returnvalue (`|CreateDelegate` :!event `DamageFlash`))
  ;[0 0 0 0.5] Setup Dynamic Material Instance
  (`/Engine/EditorBlueprintResources/StandardMacros.IsValid` _returnvalue_2
    (:`Is Valid`
      (for _index (range (`PrimitiveComponent.GetNumMaterials` _returnvalue_2))
        (bind _returnvalue_3 (`PrimitiveComponent.CreateDynamicMaterialInstance` _returnvalue_2 _index null "None"))
        (`KismetArrayLibrary.Array_Add` (`self.FlashMatArray`) _returnvalue_3)
        (bind _output (`|GetArrayItem` (`self.FlashMatArray`) _index))
        ;[0 0 0 0.5] Store Original Emissive
        (bind _returnvalue_4 (`MaterialInstanceDynamic.K2_GetVectorParameterValue` _output "EmissiveFactor"))
        (set `self.initEmissiveColor` _returnvalue_4)
        (bind _returnvalue_5 (`MaterialInstanceDynamic.K2_GetScalarParameterValue` _output "EmissiveStrength"))
        (set `self.initEmissiveStrength` _returnvalue_5)))))

(event `DamageFlash`
  (params (DamagedActor :type "Actor Object Reference") (Damage :type "Float (single-precision)") (DamageType :type "DamageType Object Reference") (InstigatedBy :type "Controller Object Reference") (DamageCauser :type "Actor Object Reference"))
  (for _array_element (`self.FlashMatArray`)
    ;[0 0 0 0.5] Set Flash Values
    (`MaterialInstanceDynamic.SetVectorParameterValue` _array_element "EmissiveFactor" (`self.FlashColor`))
    (`MaterialInstanceDynamic.SetScalarParameterValue` _array_element "EmissiveStrength" (`self.FlashIntensity`))
    (`KismetSystemLibrary.Delay` (`self.FlashDuration`))
    (for _array_element_2 (`self.FlashMatArray`)
      ;[0 0 0 0.5] Return to Original Values
      (`MaterialInstanceDynamic.SetVectorParameterValue` _array_element_2 "EmissiveFactor" (`self.initEmissiveColor`))
      (`MaterialInstanceDynamic.SetScalarParameterValue` _array_element_2 "EmissiveStrength" (`self.initEmissiveStrength`)))))