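; BP_HomingRocket is an enemy rocket that homes in on the player and kills their spaceship on contact.
; BeginPlay points the ProjectileMovement homing target at the player character's root component.
; Tick compares velocity against the direction to the player with a dot product and turns homing off once the rocket has overshot.
; Collision overlap sends a death message through INT_Player if the BP_SpaceShip is not already dead.
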(event `self.ReceiveBeginPlay`
  (bind _returnvalue (`GameplayStatics.GetPlayerCharacter` 0))
  (bind _projectilemovement (`self.ProjectileMovement`))
  (set `self.PlayerREF` _returnvalue)
  (set `ProjectileMovementComponent.bIsHomingProjectile` true _projectilemovement)
  (set `ProjectileMovementComponent.HomingAccelerationMagnitude` 3500.0 _projectilemovement)
  (set `ProjectileMovementComponent.HomingTargetComponent` (`Actor.RootComponent` _returnvalue) _projectilemovement))

(event `self.ReceiveTick`
  (params (DeltaSeconds :type "Float (single-precision)"))
  (`/Engine/EditorBlueprintResources/StandardMacros.IsValid` (`self.PlayerREF`)
    (:`Is Valid`
      (if (< (`KismetMathLibrary.Dot_VectorVector` (`KismetMathLibrary.Normal` (- (`self.K2_GetActorLocation` (`self.PlayerREF`)) (`self.K2_GetActorLocation`))) (`KismetMathLibrary.Normal` (`MovementComponent.Velocity` (`self.ProjectileMovement`)))) -0.1)
        (set `ProjectileMovementComponent.bIsHomingProjectile` false (`self.ProjectileMovement`))))
    (:`Is Not Valid`
      (`KismetSystemLibrary.PrintString` "PLAYER NOT VALID"))))

(event `self.MissileCollision.OnComponentBeginOverlap`
  (params (OverlappedComponent :type "PrimitiveComponent Object Reference") (OtherActor :type "Actor Object Reference") (OtherComp :type "PrimitiveComponent Object Reference") (OtherBodyIndex :type Integer) (bFromSweep :type Boolean) (SweepResult :type "HitResult Structure (by ref)"))
  (if (`KismetSystemLibrary.DoesImplementInterface` OtherActor "/Game/Main/Interfaces/INT_Player.INT_Player_C")
    (if (not (`/Game/Main/Player/BP_SpaceShip.IsDead` (cast `/Game/Main/Player/BP_SpaceShip` OtherActor :!pure true)))
      (message `/Game/Main/Interfaces/INT_Player.HandleDeath` OtherActor true))))

(fn `UserConstructionScript`)