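; Base enemy Blueprint for a turret-like foe that faces the player and fires homing rockets.
; LookatPlayer applies yaw-only aiming, and ShootPlayer spawns two BP_HomingRocket actors from separate muzzle points after a delay; neither is triggered within this graph.
; Damage reduces Health until death, which spawns a Niagara explosion, destroys the actor and notifies the game mode of the death and score.
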(event `self.ReceiveTick`
  (params (DeltaSeconds :type "Float (single-precision)")))

(event `/Game/Main/Interfaces/INT_Enemy.LookAtPlayer`
  (if (not (`self.IsPlayerDead`))
    (`self.K2_SetActorRotation` (`KismetMathLibrary.MakeRotator` 0.0 0.0 (.yaw (`KismetMathLibrary.FindLookAtRotation` (`self.K2_GetActorLocation`) (`self.K2_GetActorLocation` (`GameplayStatics.GetPlayerCharacter` 0))))))))

(event `/Game/Main/Interfaces/INT_Enemy.ShootPlayer`
  (bind _rocketshootlocation1 (`self.RocketShootLocation1`))
  (bind _rocketshootlocation2 (`self.RocketShootLocation2`))
  (if (not (`self.IsPlayerDead`))
    (`KismetSystemLibrary.Delay` 3.0)
    (`|SpawnActorFromClass` "/Game/Main/Enemies/HomingRocket/BP_HomingRocket.BP_HomingRocket_C" (`KismetMathLibrary.MakeTransform` (`SceneComponent.K2_GetComponentLocation` _rocketshootlocation1) (`SceneComponent.K2_GetComponentRotation` _rocketshootlocation1)) "Undefined" "MultiplyWithRoot" null null)
    (`|SpawnActorFromClass` "/Game/Main/Enemies/HomingRocket/BP_HomingRocket.BP_HomingRocket_C" (`KismetMathLibrary.MakeTransform` (`SceneComponent.K2_GetComponentLocation` _rocketshootlocation2) (`SceneComponent.K2_GetComponentRotation` _rocketshootlocation2)) "Undefined" "MultiplyWithRoot" null null)))

(event `self.ReceiveAnyDamage`
  (params (Damage :type "Float (single-precision)") (DamageType :type "DamageType Object Reference") (InstigatedBy :type "Controller Object Reference") (DamageCauser :type "Actor Object Reference"))
  (if (not (`self.IsDead`))
    (set `self.Health` (- (`self.Health`) Damage))
    (if (<= (`self.Health`) 0.0)
      (set `self.IsDead` true)
      (`self.HandleDeath`))))

(event `HandleDeath`
  (bind _returnvalue (`GameplayStatics.GetGameMode`))
  (`self.PlayFX`)
  (`self.K2_DestroyActor`)
  (message `/Game/Main/Interfaces/INT_GameMode.EnemyDied` _returnvalue)
  (message `/Game/Main/Interfaces/INT_GameMode.AddToScore` _returnvalue (`self.ScoreAmount`)))

(event `PlayFX`
  (`NiagaraFunctionLibrary.SpawnSystemAtLocation` "/Game/NiagaraExamples/FX_Explosions/NS_Explosion.NS_Explosion" (`self.K2_GetActorLocation`)))

(fn `UserConstructionScript`
  (`parent.UserConstructionScript`))