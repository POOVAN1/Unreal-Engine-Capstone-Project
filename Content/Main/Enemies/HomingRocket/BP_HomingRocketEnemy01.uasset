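; BP_HomingRocketEnemy01 is an enemy that calls LookAtPlayer and ShootPlayer every tick.
; Its MoveEnemyDownHoming event plays a timeline that lerps the actor from TopLocation to BottomLocation without sweeping.
; IsBottomHomingEnemy is cleared when the move starts and set when the timeline finishes, marking arrival at the bottom.
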(event `self.ReceiveTick`
  (params (DeltaSeconds :type "Float (single-precision)"))
  (`self.LookAtPlayer`)
  (`self.ShootPlayer`))

(event `MoveEnemyDownHoming`
  (set `self.Is_Bottom_HomingEnemy` false)
  (bind (_direction _delta) (`Timeline|Timeline` :!via `PlayFromStart`)
    (:`Update`
      (`self.K2_SetActorLocation` (`KismetMathLibrary.VLerp` (`self.TopLocation`) (`self.BottomLocation`) _delta)))
    (:`Finished`
      (set `self.Is_Bottom_HomingEnemy` true))))

(fn `UserConstructionScript`
  (`parent.UserConstructionScript`))