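; Base Blueprint for basic enemy ships that provides aiming, shooting, damage and death behavior.
; LookatPlayer yaws the ship toward the player, and ShootPlayer waits before spawning a projectile aimed at the player, flattened to the ship's height.
; Both are skipped when the player is dead, and neither is called within this graph.
; Damage drains Health until death, which spawns a Niagara explosion, destroys the actor and notifies GM_GamePlay.
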(event `self.ReceiveTick`
  (params (DeltaSeconds :type "Float (single-precision)")))

(event `/Game/Main/Interfaces/INT_Enemy.LookAtPlayer`
  (if (not (`self.IsPlayerDead`))
    (`self.K2_SetActorRotation` (`KismetMathLibrary.MakeRotator` 0.0 0.0 (.yaw (`KismetMathLibrary.FindLookAtRotation` (`self.K2_GetActorLocation`) (`self.K2_GetActorLocation` (`GameplayStatics.GetPlayerCharacter` 0))))))))

(event `/Game/Main/Interfaces/INT_Enemy.ShootPlayer`
  (bind _returnvalue (`SceneComponent.K2_GetComponentLocation` (`self.Mesh`)))
  (if (not (`self.IsPlayerDead`))
    (`KismetSystemLibrary.Delay` 4.0)
    (`|SpawnActorFromClass` "/Game/Main/Enemies/BasicEnemy/BasicEnemy_Projectile.BasicEnemy_Projectile_C" (`KismetMathLibrary.MakeTransform` _returnvalue (`KismetMathLibrary.MakeRotFromX` (`KismetMathLibrary.Normal` (- (`KismetMathLibrary.MakeVector` (.x (`SceneComponent.K2_GetComponentLocation` (`Character.Mesh` (`GameplayStatics.GetPlayerCharacter` 0)))) (.y (`SceneComponent.K2_GetComponentLocation` (`Character.Mesh` (`GameplayStatics.GetPlayerCharacter` 0)))) (.z _returnvalue)) _returnvalue)))) "Undefined" "MultiplyWithRoot" null null)))

(event `MultiPlayFX`
  (`NiagaraFunctionLibrary.SpawnSystemAtLocation` "/Game/NiagaraExamples/FX_Explosions/NS_Explosion_Medium.NS_Explosion_Medium" (`self.K2_GetActorLocation`)))

(event `self.ReceiveAnyDamage`
  (params (Damage :type "Float (single-precision)") (DamageType :type "DamageType Object Reference") (InstigatedBy :type "Controller Object Reference") (DamageCauser :type "Actor Object Reference"))
  (if (not (`self.IsDead`))
    (set `self.Health` (- (`self.Health`) Damage))
    (if (<= (`self.Health`) 0.0)
      (set `self.IsDead` true)
      (`self.HandleDeath`))))

(event `HandleDeath`
  (`self.MultiPlayFX`)
  (`self.K2_DestroyActor`)
  (`/Game/Main/GM_GamePlay.EnemyDied` (cast `/Game/Main/GM_GamePlay` (`GameplayStatics.GetGameMode`) :!pure true)))

(fn `UserConstructionScript`
  (`parent.UserConstructionScript`))