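; Basic enemy variant that patrols back and forth along the second selected spline of the level's enemy formation.
; On BeginPlay it finds and caches the BP_EnemyFormation actor.
; Each Tick it calls LookAtPlayer, advances a clamped spline distance by formation speed, and flips direction at either end.
; It then sets its location directly to that world-space point on the spline, without sweeping.
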(event `self.ReceiveBeginPlay`
  (bind _returnvalue (`GameplayStatics.GetActorOfClass` "/Game/Main/Enemies/BP_EnemyFormation.BP_EnemyFormation_C"))
  (set `self.EnemyFormationREF` _returnvalue))

(event `self.ReceiveTick`
  (params (DeltaSeconds :type "Float (single-precision)"))
  (bind _selectedspline2 (`/Game/Main/Enemies/BP_EnemyFormation.SelectedSpline2` (`self.EnemyFormationREF`)))
  (`self.LookAtPlayer`)
  (bind _output_get (set `self.SplineDistance` (`KismetMathLibrary.FClamp` (+ (`self.SplineDistance`) (* (`self.MoveDirection`) (* (`self.FormationSpeed`) DeltaSeconds))) 0.0 (`SplineComponent.GetSplineLength` _selectedspline2))))
  (if (>= (`self.SplineDistance`) (`SplineComponent.GetSplineLength` _selectedspline2))
    (set `self.MoveDirection` (* (`self.MoveDirection`) -1.0))
    (elif (<= (`self.SplineDistance`) 0.0)
      (set `self.MoveDirection` 1.0)))
  (`self.K2_SetActorLocation` (`SplineComponent.GetLocationAtDistanceAlongSpline` _selectedspline2 _output_get "World")))

(fn `UserConstructionScript`
  (`parent.UserConstructionScript`))