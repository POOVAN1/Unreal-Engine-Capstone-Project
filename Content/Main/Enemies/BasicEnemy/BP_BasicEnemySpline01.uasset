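; Basic enemy that patrols back and forth along a spline owned by the enemy formation while tracking and shooting the player.
; On BeginPlay it caches the BP_EnemyFormation actor found in the level.
; Each tick it calls LookAtPlayer and ShootPlayer, then advances a clamped distance along the formation's selected spline.
; The move direction flips at either end, and the actor snaps to that spline position without sweeping.
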(event `self.ReceiveBeginPlay`
  (bind _returnvalue (`GameplayStatics.GetActorOfClass` "/Game/Main/Enemies/BP_EnemyFormation.BP_EnemyFormation_C"))
  (set `self.EnemyFormationREF` _returnvalue))

(event `self.ReceiveTick`
  (params (DeltaSeconds :type "Float (single-precision)"))
  (bind _selectedspline (`/Game/Main/Enemies/BP_EnemyFormation.SelectedSpline` (`self.EnemyFormationREF`)))
  (`self.LookAtPlayer`)
  (`self.ShootPlayer`)
  (bind _output_get (set `self.SplineDistance` (`KismetMathLibrary.FClamp` (+ (`self.SplineDistance`) (* (`self.MoveDirection`) (* (`self.FormationSpeed`) DeltaSeconds))) 0.0 (`SplineComponent.GetSplineLength` _selectedspline))))
  (if (>= (`self.SplineDistance`) (`SplineComponent.GetSplineLength` _selectedspline))
    (set `self.MoveDirection` (* (`self.MoveDirection`) -1.0))
    (elif (<= (`self.SplineDistance`) 0.0)
      (set `self.MoveDirection` 1.0)))
  (`self.K2_SetActorLocation` (`SplineComponent.GetLocationAtDistanceAlongSpline` _selectedspline _output_get "World")))

(fn `UserConstructionScript`
  (`parent.UserConstructionScript`))