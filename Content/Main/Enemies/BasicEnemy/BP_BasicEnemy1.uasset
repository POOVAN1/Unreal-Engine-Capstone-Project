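; BP_BasicEnemy1 is a basic enemy that turns toward the player and shoots while flagged as being at the bottom position.
; Tick calls LookAtPlayer every frame and ShootPlayer only while IsBottomBasicEnemy is set.
; MoveEnemyDown_Basic clears that flag, plays a Timeline that lerps the actor from TopLocation to BottomLocation without sweep, then sets the flag when finished, so shooting pauses during the descent.
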(event `self.ReceiveBeginPlay`)

(event `self.ReceiveTick`
  (params (DeltaSeconds :type "Float (single-precision)"))
  (`self.LookAtPlayer`)
  (if (`self.IsBottom_BasicEnemy`)
    (`self.ShootPlayer`)))

(event `MoveEnemyDown_Basic`
  (set `self.IsBottom_BasicEnemy` false)
  (bind (_direction _delta) (`Timeline|Timeline` :!via `PlayFromStart`)
    (:`Update`
      (`self.K2_SetActorLocation` (`KismetMathLibrary.VLerp` (`self.TopLocation`) (`self.BottomLocation`) _delta)))
    (:`Finished`
      (set `self.IsBottom_BasicEnemy` true))))

(fn `UserConstructionScript`
  (`parent.UserConstructionScript`))