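; BP_EnemyFormation is an enemy spawner that lays out two lines of basic enemies along its spline components.
; BasicEnemySpawner updates the game mode's alive message with double the requested count, then randomly picks two different splines.
; A loop spawns BP_BasicEnemySpline01 and BP_BasicEnemySpline02 at even spacing along their respective splines, passing each its spline distance.
; A random three-way switch precedes this, but every case runs the same logic.
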(event `/Game/Main/Interfaces/INT_EnemyFormation.BasicEnemySpawner`
  (params (EnemiesAlive :type Integer))
  (switch `int` (`KismetMathLibrary.RandomIntegerInRange` 0 2)
    (:`0`
      _)
    (:`1`
      _)
    (:`2`
      _))
  (set `self.EnemiesAlive` EnemiesAlive)
  (message `/Game/Main/Interfaces/INT_GameMode.UpdateEnemiesAlive` (`GameplayStatics.GetGameMode`) (* (`self.EnemiesAlive`) 2))
  (bind _output_get (set `self.AvailableSplines` (`self.K2_GetComponentsByClass` "/Script/Engine.SplineComponent")))
  (bind _output_get_2 (set `self.SelectedSpline` (`KismetArrayLibrary.Array_Random` _output_get)))
  (`KismetArrayLibrary.Array_RemoveItem` (`self.AvailableSplines`) _output_get_2)
  (set `self.SelectedSpline2` (`KismetArrayLibrary.Array_Random` (`self.AvailableSplines`)))
  (for _index (range (`self.EnemiesAlive`))
    (bind _output_get_3 (set `self.EnemyDistance` (* _index (`self.EnemySpacing`))))
    (`|SpawnActorFromClass` "/Game/Main/Enemies/BasicEnemy/BP_BasicEnemySpline01.BP_BasicEnemySpline01_C" (`KismetMathLibrary.MakeTransform` (`SplineComponent.GetLocationAtDistanceAlongSpline` (`self.SelectedSpline`) (`self.EnemyDistance`) "World")) "Undefined" "MultiplyWithRoot" null _output_get_3 (0.0 0.0 0.0) (0.0 0.0 0.0) null)
    (`|SpawnActorFromClass` "/Game/Main/Enemies/BasicEnemy/BP_BasicEnemySpline02.BP_BasicEnemySpline02_C" (`KismetMathLibrary.MakeTransform` (`SplineComponent.GetLocationAtDistanceAlongSpline` (`self.SelectedSpline2`) (`self.EnemyDistance`) "World")) "Undefined" "MultiplyWithRoot" null _output_get_3 (0.0 0.0 0.0) (0.0 0.0 0.0) null)))

(fn `UserConstructionScript`)