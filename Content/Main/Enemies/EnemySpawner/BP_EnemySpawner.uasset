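; BP_EnemySpawner spawns wave-one basic enemies at spawn points, with a landing indicator marking where each comes down.
; Wave1Spawner frees all points, then randomly picks one per enemy without repeats, capping the count at the available points.
; Each spawn flashes an indicator at the point's bottom location and starts the enemy moving down.
; Wave 2 is an empty stub, and the timer-based spawn path is unwired.
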(event `self.ReceiveBeginPlay`)

(event `/Game/Main/Interfaces/INT_EnemySpawner.Wave1Spawner`
  (params (EnemiesRemaining :type Integer))
  (bind _currentspawnpoint (`self.CurrentSpawnPoint`))
  (bind _output (`|GetArrayItem` (`self.AvailableSpawnPoints`) (`self.RandomIndex`)))
  (set `self.EnemiesRemaining` EnemiesRemaining)
  (`KismetArrayLibrary.Array_Clear` (`self.AvailableSpawnPoints`))
  (for _array_element (`self.SpawnPoints`)
    (set `/Game/Main/Enemies/EnemySpawner/BP_SpawnPoints.IsOccupied` false _array_element))
  (for _array_element_2 (`self.SpawnPoints`)
    (if (not (`/Game/Main/Enemies/EnemySpawner/BP_SpawnPoints.IsOccupied` _array_element_2))
      (`KismetArrayLibrary.Array_Add` (`self.AvailableSpawnPoints`) _array_element_2)))
  (for _ (range (`self.EnemiesRemaining`))
    (if (> (`KismetArrayLibrary.Array_Length` (`self.AvailableSpawnPoints`)) 0)
      (set `self.RandomIndex` (`KismetMathLibrary.RandomIntegerInRange` 0 (- (`KismetArrayLibrary.Array_Length` (`self.AvailableSpawnPoints`)) 1)))
      (bind _output_get (set `self.CurrentSpawnPoint` _output))
      (`/Engine/EditorBlueprintResources/StandardMacros.IsValid` _output_get
        (:`Is Valid`
          (`self.DrawSpawnCircle`)
          (bind _returnvalue (`|SpawnActorFromClass` "/Game/Main/Enemies/BasicEnemy/BP_BasicEnemy1.BP_BasicEnemy1_C" (`self.GetTransform` (`self.CurrentSpawnPoint`)) "Undefined" "MultiplyWithRoot" null (`/Game/Main/Enemies/EnemySpawner/BP_SpawnPoints.TopLocation` _currentspawnpoint) (`KismetMathLibrary.MakeVector` (.x (`/Game/Main/Enemies/EnemySpawner/BP_SpawnPoints.BottomLocation` _currentspawnpoint)) (.y (`/Game/Main/Enemies/EnemySpawner/BP_SpawnPoints.BottomLocation` _currentspawnpoint)) 92.0) null))
          (set `/Game/Main/Enemies/EnemySpawner/BP_SpawnPoints.IsOccupied` true _output)
          (`KismetArrayLibrary.Array_Remove` (`self.AvailableSpawnPoints`) (`self.RandomIndex`))
          (`/Game/Main/Enemies/BasicEnemy/BP_BasicEnemy1.MoveEnemyDown_Basic` _returnvalue))
        (:`Is Not Valid`
          (`KismetSystemLibrary.PrintString` "ERROR"))))))

(event `Wave2_Spawner`)

(event `DrawSpawnCircle`
  (bind _returnvalue (`|SpawnActorFromClass` "/Game/Main/Enemies/EnemySpawnMarker/BP_LandingIndicator.BP_LandingIndicator_C" (`KismetMathLibrary.MakeTransform` (`KismetMathLibrary.MakeVector` (.x (`/Game/Main/Enemies/EnemySpawner/BP_SpawnPoints.BottomLocation` (`self.CurrentSpawnPoint`))) (.y (`/Game/Main/Enemies/EnemySpawner/BP_SpawnPoints.BottomLocation` (`self.CurrentSpawnPoint`))) 92.0)) "Undefined" "MultiplyWithRoot" null null))
  (`/Game/Main/Enemies/EnemySpawnMarker/BP_LandingIndicator.PlayFlash` _returnvalue))

(event `SpawnNextEnemy_Wave1`
  (bind _returnvalue (`|SpawnActorFromClass` "/Game/Main/Enemies/BasicEnemy/BP_BasicEnemy1.BP_BasicEnemy1_C" (`KismetMathLibrary.MakeTransform` (`self.K2_GetActorLocation` (`KismetArrayLibrary.Array_Random` (`self.SpawnPoints`)))) "Undefined" "MultiplyWithRoot" null (0.0 0.0 0.0) (0.0 0.0 0.0) null))
  (`KismetSystemLibrary.PrintString` (`KismetSystemLibrary.GetDisplayName` _returnvalue))
  (set `self.EnemiesRemainingToSpawn` (- 1 (`self.EnemiesRemainingToSpawn`)))
  (if (<= (`self.EnemiesRemainingToSpawn`) 0)
    (`KismetSystemLibrary.K2_ClearTimer` null "Wave1_Spawner")))

(fn `UserConstructionScript`)