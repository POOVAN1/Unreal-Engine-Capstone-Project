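; Game mode for gameplay that runs an enemy wave loop through the level's BP_EnemySpawner, found at BeginPlay.
; StartWave advances the wave counter, sets the alive count and, after a short delay, messages the spawner; only the first two waves are defined, both using the same spawner call.
; EnemyDied decrements the count and, when none remain, WaveCompleted prints a message and starts the next wave.
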(event `self.ReceiveBeginPlay`
  (bind _outactors (`GameplayStatics.GetAllActorsOfClass` "/Game/Main/Enemies/EnemySpawner/BP_EnemySpawner.BP_EnemySpawner_C"))
  (set `self.EnemySpawner` (`|GetArrayItem` _outactors))
  (`self.StartWave`))

(event `StartWave`
  (bind _enemyspawner (`self.EnemySpawner`))
  (bind _output_get (set `self.CurrentWave` (+ (`self.CurrentWave`) 1)))
  (set `self.WaveInProgress` true)
  (switch `int` _output_get
    (:`1`
      (bind _output_get_2 (set `self.EnemiesAlive` 10))
      (`KismetSystemLibrary.Delay` 5.0)
      (message `/Game/Main/Interfaces/INT_EnemySpawner.Wave1Spawner` _enemyspawner _output_get_2))
    (:`2`
      (bind _output_get_3 (set `self.EnemiesAlive` 10))
      (`KismetSystemLibrary.Delay` 5.0)
      (message `/Game/Main/Interfaces/INT_EnemySpawner.Wave1Spawner` _enemyspawner _output_get_3))))

(event `EnemyDied`
  (bind _output_get (set `self.EnemiesAlive` (- (`self.EnemiesAlive`) 1)))
  (`KismetSystemLibrary.PrintString` (`KismetStringLibrary.Conv_IntToString` _output_get))
  (if (<= (`self.EnemiesAlive`) 0)
    (`self.WaveCompleted`)))

(event `WaveCompleted`
  (`KismetSystemLibrary.PrintString` "Wave Completed")
  (`self.StartWave`))

(fn `UserConstructionScript`)